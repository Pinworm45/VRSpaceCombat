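; VR player controller that switches possession between the carrier, its turrets, fighters and miners, and runs the settings menu and music player.
; BeginPlay caches the carrier and Lancer references, creates the menu widget and starts a looping timer that advances songs when they end.
; Input cycles turrets through the Lancer and units through the Fighters and Miners arrays.
; A Tick-fed gate times the NextSong press, so a tap skips and a hold stops playback.
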(event Custom|UpdateTimeElapsed
  ;[1 1 1] Update Time Elapsed
  (if (Variables|Default|GetSongIsPlaying)
    (bind _result (Math|Float|IncrementFloat (Variables|Default|GetTimeElapsed))
      (:%20%20
        (if (>= _result (Variables|Default|GetSongDuration))
          (CallFunction|NextSong))))))

(event EventTick
  (params (DeltaSeconds :type Float%20%28single-precision%29))
  ;[1 1 1] Music Commands
  (Utilities|FlowControl|Gate true
    (:Exit
      (Variables|Default|SetNextSongHeld (+ (Variables|Default|GetNextSongHeld) DeltaSeconds)))))

(event EventBeginPlay
  ;[1 1 1] Begin play, set vars
  (bind _asbase_carrier (Utilities|Casting|CastToBase_Carrier (Game|Player|GetPlayerPawn 0))
    (:then
      (bind _output_get (Variables|Default|SetCarrier _asbase_carrier))
      (bind _aspawn_carrier_lancer (Utilities|Casting|CastToPawn_Carrier_Lancer _output_get))
      (Variables|Default|SetLancer _aspawn_carrier_lancer))
    (:CastFailed
      (bind _outactors (Actor|GetAllActorsOfClass "/Game/Blueprints/Ships/Base_Carrier.Base_Carrier_C"))
      (bind _output_get_2 (Variables|Default|SetCarrier (Utilities|Array|Get(acopy) _outactors)))
      (bind _aspawn_carrier_lancer_2 (Utilities|Casting|CastToPawn_Carrier_Lancer _output_get_2))
      (Variables|Default|SetLancer _aspawn_carrier_lancer_2)))
  (bind _game_settings (Utilities|GetGameSettings (Game|GetGameInstance)))
  (Variables|Default|SetGame%20Settings _game_settings)
  (bind _returnvalue (UserInterface|CreateWidget "/Game/QualityMenu/HUD_UMG_Classic/ClassicSettingsMain.ClassicSettingsMain_C" 0 false true (Variables|Default|GetActionManager)))
  (bind _output_get_3 (Variables|Default|SetSettingsMenu _returnvalue))
  (UserInterface|Viewport|AddtoViewport _output_get_3 1)
  (bind _output_get_4 (Variables|Default|SetSongIndex (Math|Random|RandomIntegerinRange 0 (Utilities|Array|LastIndex (Variables|Default|GetComfySongs)))))
  (Variables|Default|SetTimeElapsed 0.0)
  (Variables|Default|SetSongIsPlaying false)
  (Utilities|Time|SetTimerbyEvent (delegate Custom|UpdateTimeElapsed) 1.0 true))

(event Input|ActionEvents|InputActionNextWeaponOrTurret
  (params (Key :type Key%20Structure :default "AnyKey"))
  (bind _lancer (Variables|Default|GetLancer))
  ;[1 1 1] Turrets
  (:Pressed
    (Default|PossessTurret _lancer (+ (Variables|/Game/Blueprints/Ships/Pawn_Carrier_Lancer.Pawn_Carrier_Lancer_C|GetPozzedTurret _lancer) 1))))

(event Input|ActionEvents|InputActionSelectFighters
  (params (Key :type Key%20Structure :default "AnyKey"))
  ;[1 1 1] Select Fighters
  (:Pressed
    (CallFunction|SelectFighters)))

(event Input|ActionEvents|InputActionSelectMiners
  (params (Key :type Key%20Structure :default "AnyKey"))
  ;[1 1 1] Select Miners
  (:Pressed
    (CallFunction|SelectMiners)))

(event Input|ActionEvents|InputActionPreviousWeaponOrTurret
  (params (Key :type Key%20Structure :default "AnyKey"))
  (bind _lancer (Variables|Default|GetLancer))
  ;[1 1 1] Turrets
  (:Pressed
    (Default|PossessTurret _lancer (- (Variables|/Game/Blueprints/Ships/Pawn_Carrier_Lancer.Pawn_Carrier_Lancer_C|GetPozzedTurret _lancer) 1))))

(event Input|ActionEvents|InputActionMenu
  (params (Key :type Key%20Structure :default "AnyKey"))
  (bind _settingsmenu (Variables|Default|GetSettingsMenu))
  ;[1 1 1] Menu
  (:Pressed
    (if (Variables|/Game/QualityMenu/HUD_UMG_Classic/ClassicSettingsMain.ClassicSettingsMain_C|GetIs%20Menu%20Open _settingsmenu)
      (Default|CloseMenu _settingsmenu)
      (else
        (Default|OpenMenu _settingsmenu)))))

(event Input|ActionEvents|InputActionNextSong
  (params (Key :type Key%20Structure :default "AnyKey"))
  ;[1 1 1] Music Commands
  (:Pressed
    (Utilities|FlowControl|Sequence
      (:then_0
        (Utilities|FlowControl|DoOnce false :!label _label
          (:Completed
            (Variables|Default|SetNextSongHeld 0.0))))
      (:then_1
        (Utilities|FlowControl|Gate true) ; enters at Open
      )))
  (:Released
    (Utilities|FlowControl|Sequence
      (:then_0
        (Utilities|FlowControl|Gate true) ; enters at Close
      )
      (:then_1
        (if (>= (Variables|Default|GetNextSongHeld) 0.75)
          (CallFunction|StopMusic)
          (else
            (CallFunction|NextSong))))
      (:then_2
        (goto _label Reset)))))

(event Input|ActionEvents|InputActionSelectCarrier
  (params (Key :type Key%20Structure :default "AnyKey"))
  ;[1 1 1] Select Carrier
  (:Pressed
    (CallFunction|SelectCarrier)))

(fn ConstructionScript)

(fn SelectCarrier
  (bind _lancer (Variables|Default|GetLancer))
  (Utilities|IsValid _lancer
    (:Is%20Valid
      (Pawn|Possess _lancer))
    (:Is%20Not%20Valid
      (Pawn|Possess (Variables|Default|GetCarrier)))))

(fn SelectFighters
  (bind _fighters (Variables|Default|GetFighters))
  (Variables|Default|SetUnitToPoz 0)
  (for (_array_element _array_index) _fighters
    (if (== (Pawn|GetController _array_element) self)
      (Variables|Default|SetUnitToPoz (+ _array_index 1))))
  (if (== (Variables|Default|GetUnitToPoz) (+ (Utilities|Array|LastIndex _fighters) 1))
    (Pawn|Possess (Utilities|Array|Get(acopy) _fighters))
    (else
      (Pawn|Possess (Utilities|Array|Get(acopy) _fighters (Variables|Default|GetUnitToPoz))))))

(fn SelectMiners
  (bind _miners (Variables|Default|GetMiners))
  (Variables|Default|SetUnitToPoz 0)
  (for (_array_element _array_index) _miners
    (if (== (Pawn|GetController _array_element) self)
      (Variables|Default|SetUnitToPoz (+ _array_index 1))))
  (if (== (Variables|Default|GetUnitToPoz) (+ (Utilities|Array|LastIndex _miners) 1))
    (Pawn|Possess (Utilities|Array|Get(acopy) _miners))
    (else
      (Pawn|Possess (Utilities|Array|Get(acopy) _miners (Variables|Default|GetUnitToPoz))))))

(fn NextSong
  (Utilities|IsValid (Variables|Default|GetPlayingSong)
    (:Is%20Valid
      (Audio|Components|Audio|Stop (Variables|Default|GetPlayingSong))
      (Components|DestroyComponent (Variables|Default|GetPlayingSong)))
    (:Is%20Not%20Valid
      _))
  (bind _result (Math|Integer|IncrementInt (Variables|Default|GetSongIndex))
    (:%20%20
      (if (> _result (Utilities|Array|LastIndex (Variables|Default|GetComfySongs)))
        (Variables|Default|SetSongIndex 0))
      (bind _returnvalue (Audio|SpawnSound2D (Utilities|Array|Get(acopy) (Variables|Default|GetComfySongs) (Variables|Default|GetSongIndex))))
      (bind _output_get (Variables|Default|SetPlayingSong _returnvalue))
      (Variables|Default|SetSongString (Utilities|Text|ToText(String) (Utilities|GetObjectName (Utilities|Array|Get(acopy) (Variables|Default|GetComfySongs) (Variables|Default|GetSongIndex)))))
      (Variables|Default|SetSongDuration (Variables|/Script/Engine.SoundBase|GetDuration (Variables|/Script/Engine.AudioComponent|GetSound _output_get)))
      (Variables|Default|SetTimeElapsed 0.0)
      (Variables|Default|SetSongIsPlaying true))))

(fn StopMusic
  (bind _playingsong (Variables|Default|GetPlayingSong))
  (Utilities|IsValid _playingsong
    (:Is%20Valid
      (Audio|Components|Audio|Stop _playingsong)
      (Components|DestroyComponent _playingsong)
      (Variables|Default|SetSongIsPlaying false))))