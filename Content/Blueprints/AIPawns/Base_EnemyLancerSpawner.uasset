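; Enemy lancer spawner that periodically launches AI fighter pawns into the level.
; On BeginPlay a looping five-second timer fires a spawn event, which a FlipFlop alternates between two arrow components.
; Each spawn creates a Base_Fighter_AIBT running BT_EnemyFighter at that arrow's transform, ignoring collision, and copies the spawner's actor tags onto the new pawn.
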(event Custom|SpawnAIFighter
  (bind _arrow_0 (Variables|Default|GetArrow_0))
  (bind _arrow1 (Variables|Default|GetArrow1))
  (bind _returnvalue (Transformation|GetWorldTransform _arrow1))
  (bind _returnvalue_2 (Transformation|GetWorldTransform _arrow_0))
  (bind (_location _rotation) (Math|Transform|BreakTransform _returnvalue))
  (bind (_location_2 _rotation_2) (Math|Transform|BreakTransform _returnvalue_2))
  (Utilities|FlowControl|FlipFlop
    (:A
      (bind _returnvalue_3 (AI|SpawnAIFromClass "/Game/Blueprints/AIPawns/Base_Fighter_AIBT.Base_Fighter_AIBT_C" "/Game/Blueprints/AIPawns/FighterAI/BT_EnemyFighter.BT_EnemyFighter" _location_2 _rotation_2 true))
      (Variables|/Script/Engine.Actor|SetTags _returnvalue_3 (Variables|Default|GetTags)))
    (:B
      (bind _returnvalue_4 (AI|SpawnAIFromClass "/Game/Blueprints/AIPawns/Base_Fighter_AIBT.Base_Fighter_AIBT_C" "/Game/Blueprints/AIPawns/FighterAI/BT_EnemyFighter.BT_EnemyFighter" _location _rotation true))
      (Variables|/Script/Engine.Actor|SetTags _returnvalue_4 (Variables|Default|GetTags)))))

(event EventBeginPlay
  (|CallParentFunction)
  (Utilities|Time|SetTimerbyEvent (delegate Custom|SpawnAIFighter) 5.0 true))

(fn ConstructionScript
  (|CallParentFunction))