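; Base AI fighter ship pawn, set up for a blackboard-driven AI, that fights for one of two teams identified by its first actor tag.
; BeginPlay passes the patrol flag to the blackboard, applies the team texture and seeds Targets from DetectSphere, whose overlaps then update the list.
; FireGuns spawns team-tagged projectiles, randomly blending aim between gun-arrow direction and target.
; Lethal damage spawns a DM_UFO actor and explosion, then destroys the pawn.
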(event OnComponentBeginOverlap(DetectSphere)
  (params (OverlappedComponent :type Primitive%20Component%20Object%20Reference) (OtherActor :type Actor%20Object%20Reference) (OtherComp :type Primitive%20Component%20Object%20Reference) (OtherBodyIndex :type Integer) (bFromSweep :type Boolean) (SweepResult :type Hit%20Result%20Structure%20%28by%20ref%29))
  (Utilities|Casting|CastToPawn_Fighter_Phys OtherActor)
  (if (not (Utilities|Name|Equal(Name) (Utilities|Array|Get(acopy) (Variables|Default|GetTags)) (Utilities|Array|Get(acopy) (Variables|/Script/Engine.Actor|GetTags OtherActor))))
    (Utilities|Array|Add (Variables|Default|GetTargets) OtherActor)))

(event OnComponentEndOverlap(DetectSphere)
  (params (OverlappedComponent :type Primitive%20Component%20Object%20Reference) (OtherActor :type Actor%20Object%20Reference) (OtherComp :type Primitive%20Component%20Object%20Reference) (OtherBodyIndex :type Integer))
  (Utilities|Casting|CastToPawn_Fighter_Phys OtherActor
    (:then
      (Utilities|Array|RemoveItem (Variables|Default|GetTargets) 0))
    (:CastFailed
      (if (not (Utilities|Name|Equal(Name) (Utilities|Array|Get(acopy) (Variables|Default|GetTags)) (Utilities|Array|Get(acopy) (Variables|/Script/Engine.Actor|GetTags OtherActor))))
        (Utilities|Array|RemoveItem (Variables|Default|GetTargets) 0)))))

(event EventBeginPlay
  (AI|Components|Blackboard|SetValueasBool (AI|GetBlackboard 0) (Variables|Default|GetPatrolKey) (Variables|Default|GetPatrol))
  (Utilities|FlowControl|Delay 0.02)
  (bind _returnvalue (Rendering|Material|CreateDynamicMaterialInstance (Variables|Default|GetShipMesh) 0 "/Game/Meshes/Textures/Fighter_Mat.Fighter_Mat" :!class /Script/Engine.PrimitiveComponent))
  (switch name (Utilities|Array|Get(acopy) (Variables|Default|GetTags))
    (:team1
      (Rendering|Material|SetTextureParameterValue _returnvalue "MatPara2d" "/Game/Meshes/Textures/Texture_Fighter_Red.Texture_Fighter_Red"))
    (:team2
      (Rendering|Material|SetTextureParameterValue _returnvalue "MatPara2d" "/Game/Meshes/Textures/Texture_Fighter_Yellow.Texture_Fighter_Yellow")))
  (for _array_element (Collision|GetOverlappingActors (Variables|Default|GetDetectSphere) 0 :!class /Script/Engine.PrimitiveComponent)
    (if (not (Actor|ActorHasTag _array_element (Utilities|Array|Get(acopy) (Variables|Default|GetTags))))
      (Utilities|Array|Add (Variables|Default|GetTargets) _array_element))))

(event Game|Damage|EventAnyDamage
  (params (Damage :type Float%20%28single-precision%29) (DamageType :type Damage%20Type%20Object%20Reference) (InstigatedBy :type Controller%20Object%20Reference) (DamageCauser :type Actor%20Object%20Reference))
  (bind _scene (Variables|Default|GetScene))
  (bind _returnvalue (Transformation|GetWorldTransform _scene))
  (bind (_location _rotation) (Math|Transform|BreakTransform _returnvalue))
  ;[1 1 1] Damage / death
  (bind _output_get (Variables|Default|SetHealth (- (Variables|Default|GetHealth) Damage)))
  (if (<= _output_get 0.0)
    (Game|SpawnActorfromClass "/Game/Blueprints/AIPawns/DM_UFO.DM_UFO_C" (Math|Transform|MakeTransform _location _rotation "15.000000,15.000000,10.000000") "AlwaysSpawn" 0 0)
    (bind _returnvalue_2 (Effects|SpawnEmitteratLocation "/Game/Particles/P_Explosion.P_Explosion" (Transformation|GetActorLocation)))
    (Transformation|SetWorldScale3D _returnvalue_2 "15.000000,15.000000,15.000000")
    (Actor|DestroyActor)))

(fn ConstructionScript
  (|CallParentFunction))

(fn FireGuns
  (params (target :type Actor%20Object%20Reference))
  (bind _arrow (Variables|Default|GetArrow))
  (bind _returnvalue (Transformation|GetWorldTransform _arrow))
  (bind (_location _rotation _scale) (Math|Transform|BreakTransform _returnvalue))
  (bind _returnvalue_2 (Game|SpawnActorfromClass "/Game/Blueprints/Weapons/EnemyProjectile.EnemyProjectile_C" (Math|Transform|MakeTransform _location (Math|Rotator|Lerp(Rotator) _rotation (Math|Rotator|FindLookatRotation _location (Transformation|GetActorLocation target)) (Math|Random|RandomFloatinRange 0.0 1.0)) _scale) "AlwaysSpawn" 0 0))
  (Variables|/Script/Engine.Actor|SetTags _returnvalue_2 (Variables|Default|GetTags)))