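; Ship actor that follows the nearest SplinePath in the level, matching its location and rotation along the spline.
; BeginPlay picks the closest path and caches the distance of each spline point.
; While FollowsSpline is set, Tick advances by an FInterpTo step scaled by spline length, flagging WaitTilNextDestination near intermediate points.
; A gate stops movement near the final point; MoveToNextSpline is an empty stub.
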(event EventBeginPlay
  (bind _segmentlocations (Variables|Default|GetSegmentLocations))
  (bind _outactors (Actor|GetAllActorsOfClass "/Game/Blueprints/SplinePath.SplinePath_C"))
  (for _array_element _outactors
    (if (< (Transformation|GetDistanceTo _array_element) (Variables|Default|GetDistanceToSpline))
      (Variables|Default|SetDistanceToSpline (Transformation|GetDistanceTo _array_element))
      (Variables|Default|SetNearestSplinePath _array_element)))
  (Utilities|Array|Clear _segmentlocations)
  (for _index (range 0 (Spline|GetNumberOfSplinePoints (Variables|/Game/Blueprints/SplinePath.SplinePath_C|GetSpline (Variables|Default|GetNearestSplinePath))))
    (Utilities|Array|Add _segmentlocations (Spline|GetDistanceAlongSplineatSplinePoint (Variables|/Game/Blueprints/SplinePath.SplinePath_C|GetSpline (Variables|Default|GetNearestSplinePath)) _index))))

(event EventTick
  (params (DeltaSeconds :type Float%20%28single-precision%29))
  (bind _nearestsplinepath (Variables|Default|GetNearestSplinePath))
  (bind _spline (Variables|/Game/Blueprints/SplinePath.SplinePath_C|GetSpline _nearestsplinepath))
  (Utilities|FlowControl|Gate false :!label _label
    (:Exit
      (if (Variables|Default|GetFollowsSpline)
        (bind _output_get (Variables|Default|SetCurrentDistance (+ (Math|Interpolation|FInterpTo 0.0 (Spline|GetSplineLength (Variables|/Game/Blueprints/SplinePath.SplinePath_C|GetSpline (Variables|Default|GetNearestSplinePath))) DeltaSeconds (Variables|Default|GetSpeed)) (stale _output_get))))
        (Transformation|SetActorLocationAndRotation (Spline|GetLocationatDistanceAlongSpline _spline _output_get "World") (Spline|GetRotationatDistanceAlongSpline _spline _output_get "World"))
        (if (< (- (Utilities|Array|Get(acopy) (Variables|Default|GetSegmentLocations) (+ (Variables|Default|GetCurrSplineNdx) 1)) (Variables|Default|GetCurrentDistance)) (Variables|Default|GetDistanceTillNextShift))
          (Math|Integer|CompareInt (+ (Variables|Default|GetCurrSplineNdx) 1) (- (Utilities|Array|Length (Variables|Default|GetSegmentLocations)) 1)
            (:>
              (goto _label Close))
            (:==
              (goto _label Close))
            (:<
              (Variables|Default|SetCurrSplineNdx (+ (Variables|Default|GetCurrSplineNdx) 1))
              (Variables|Default|SetWaitTilNextDestination true))))))))

(fn ConstructionScript)

(fn MovetoNextSpline)