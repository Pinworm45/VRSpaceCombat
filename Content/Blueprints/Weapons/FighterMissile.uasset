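; FighterMissile is a homing missile actor that chases a Target and damages it on impact.
; Tick moves it forward by a fixed, swept per-frame offset, not scaled by delta time, and smoothly rotates it toward the Target with RInterpTo.
; A looping timer spawns engine-glow emitters as a trail.
; Overlapping the Target applies Damage, and either that hit or an invalid Target spawns a scaled-up explosion and destroys the missile.
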(event OnComponentBeginOverlap(Sphere)
  (params (OverlappedComponent :type Primitive%20Component%20Object%20Reference) (OtherActor :type Actor%20Object%20Reference) (OtherComp :type Primitive%20Component%20Object%20Reference) (OtherBodyIndex :type Integer) (bFromSweep :type Boolean) (SweepResult :type Hit%20Result%20Structure%20%28by%20ref%29))
  (bind _target (Variables|Default|GetTarget))
  ;[1 1 1] Overlap
  (if (== OtherActor _target)
    (bind _returnvalue (Effects|SpawnEmitteratLocation "/Game/Particles/P_Explosion.P_Explosion" (Transformation|GetActorLocation)))
    (Transformation|SetWorldScale3D _returnvalue "5.000000,5.000000,5.000000")
    (Game|Damage|ApplyDamage _target (Variables|Default|GetDamage) 0 0)
    (Actor|DestroyActor)))

(event Custom|SpawnParticleTrail
  ;[1 1 1] Trail emitter
  (Effects|SpawnEmitteratLocation "/Game/Particles/P_EngineGlow.P_EngineGlow" (Transformation|GetActorLocation)))

(event EventTick
  (params (DeltaSeconds :type Float%20%28single-precision%29))
  (bind _target (Variables|Default|GetTarget))
  ;[1 1 1] Check if valid target, if so move forward and interp to taget
  (Utilities|IsValid _target
    (:Is%20Valid
      (Transformation|AddActorLocalOffset "250.000000, 0, 0" true false)
      (Utilities|IsValid _target
        (:Is%20Valid
          (Transformation|SetActorRotation (Math|Interpolation|RInterpTo (Transformation|GetActorRotation) (Math|Rotator|FindLookatRotation (Transformation|GetActorLocation) (Transformation|GetActorLocation _target)) DeltaSeconds 5.0)))
        (:Is%20Not%20Valid
          (bind _returnvalue (Effects|SpawnEmitteratLocation "/Game/Particles/P_Explosion.P_Explosion" (Transformation|GetActorLocation) :!label _label))
          (Transformation|SetWorldScale3D _returnvalue "5.000000,5.000000,5.000000")
          (Actor|DestroyActor))))
    (:Is%20Not%20Valid
      (goto _label))))

(event EventBeginPlay
  ;[1 1 1] Trail emitter
  (Utilities|Time|SetTimerbyEvent (delegate Custom|SpawnParticleTrail) 0.033 true))

(fn ConstructionScript)